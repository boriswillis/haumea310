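; BP_pot is an interactable pot actor that shows a prompt to the player and plays a success moment on interaction.
; It creates the P1_Interact widget on BeginPlay, shows it while player character 0 overlaps its sphere, and clears all widgets on exit.
; Interact uses a FlipFlop with only A wired, so every other call shows the Sucess widget with a victory sound, then clears all widgets after a short delay.
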(event OnComponentBeginOverlap(Sphere)
  (params (OverlappedComponent :type Primitive%20Component%20Object%20Reference) (OtherActor :type Actor%20Object%20Reference) (OtherComp :type Primitive%20Component%20Object%20Reference) (OtherBodyIndex :type Integer) (bFromSweep :type Boolean) (SweepResult :type Hit%20Result%20Structure%20%28by%20ref%29))
  (if (== OtherActor (Game|GetPlayerCharacter 0))
    (UserInterface|Viewport|AddtoViewport (Variables|Default|Getpotint) 0)))

(event OnComponentEndOverlap(Sphere)
  (params (OverlappedComponent :type Primitive%20Component%20Object%20Reference) (OtherActor :type Actor%20Object%20Reference) (OtherComp :type Primitive%20Component%20Object%20Reference) (OtherBodyIndex :type Integer))
  (if (== (Game|GetPlayerCharacter 0) OtherActor)
    (Widget|RemovefromParent (Variables|Default|Getpotint))
    (Viewport|RemoveAllWidgets)))

(event EventBeginPlay
  (bind _returnvalue (UserInterface|CreateWidget "/Game/BunnyInteraction/P1_Interact.P1_Interact_C"))
  (Variables|Default|Setpotint _returnvalue))

(event EventInteract
  (Utilities|FlowControl|FlipFlop
    (:A
      (Viewport|RemoveAllWidgets)
      (bind _returnvalue (UserInterface|CreateWidget "/Game/UI/Sucess.Sucess_C"))
      (UserInterface|Viewport|AddtoViewport _returnvalue 0)
      (Audio|PlaySound2D "/Game/Music/Victory_Cue.Victory_Cue" 1.0 1.0 0.0 0 0)
      (Utilities|FlowControl|Delay 2.5)
      (Viewport|RemoveAllWidgets))))

(fn ConstructionScript)