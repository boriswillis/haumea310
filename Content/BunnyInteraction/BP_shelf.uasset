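; BP_shelf is an interactable shelf that shows an interact prompt and opens an ingredient menu.
; A P1_Interact widget is created at BeginPlay, then shown or removed as the first player's character enters or leaves the Box trigger, with exit clearing all widgets.
; The Interact event runs through a FlipFlop with only A wired, so every other call clears widgets and displays a newly created menu.
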(event OnComponentBeginOverlap(Box)
  (params (OverlappedComponent :type Primitive%20Component%20Object%20Reference) (OtherActor :type Actor%20Object%20Reference) (OtherComp :type Primitive%20Component%20Object%20Reference) (OtherBodyIndex :type Integer) (bFromSweep :type Boolean) (SweepResult :type Hit%20Result%20Structure%20%28by%20ref%29))
  (if (== OtherActor (Game|GetPlayerCharacter 0))
    (UserInterface|Viewport|AddtoViewport (Variables|Default|GetInteracgWidge) 0)))

(event OnComponentEndOverlap(Box)
  (params (OverlappedComponent :type Primitive%20Component%20Object%20Reference) (OtherActor :type Actor%20Object%20Reference) (OtherComp :type Primitive%20Component%20Object%20Reference) (OtherBodyIndex :type Integer))
  (if (== (Game|GetPlayerCharacter 0) OtherActor)
    (Widget|RemovefromParent (Variables|Default|GetInteracgWidge))
    (Viewport|RemoveAllWidgets)))

(event EventInteract
  (Utilities|FlowControl|FlipFlop
    (:A
      (Viewport|RemoveAllWidgets)
      (bind _returnvalue (UserInterface|CreateWidget "/Game/UI/IngredientMenu.IngredientMenu_C"))
      (bind _output_get (Variables|Default|Setinteractfood _returnvalue))
      (UserInterface|Viewport|AddtoViewport _output_get 0))))

(event EventBeginPlay
  (bind _returnvalue (UserInterface|CreateWidget "/Game/BunnyInteraction/P1_Interact.P1_Interact_C"))
  (Variables|Default|SetInteracgWidge _returnvalue))

(fn ConstructionScript)